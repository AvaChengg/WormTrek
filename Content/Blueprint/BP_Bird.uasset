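; BP_Bird is an actor that moves its Bird component to a FinalLocation point, then removes itself.
; On BeginPlay, the MoveTo timeline lerps Bird's world location toward FinalLocation, starting each update from the current position rather than a stored start, so steps compound.
; Once Bird is within a small tolerance of the target, the actor is destroyed after a short delay.
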(event EventBeginPlay
  ;[1 1 1] Move to the target point
  (bind _move (Timeline|MoveTo PlayFromStart)
    (:Update
      (Transformation|SetWorldLocation (Variables|Default|GetBird) (Math|Vector|Lerp(Vector) (Transformation|GetWorldLocation (Variables|Default|GetBird)) (Transformation|GetWorldLocation (Variables|Default|GetFinalLocation)) _move) false false)
      (if (Math|Vector|Equal(Vector) (Transformation|GetWorldLocation (Variables|Default|GetBird)) (Transformation|GetWorldLocation (Variables|Default|GetFinalLocation)) 1.0)
        (Utilities|FlowControl|Delay 1.0)
        (Actor|DestroyActor)))))

(fn ConstructionScript)