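; BP_Leaf is a physics-driven leaf-and-stick puzzle piece that reacts to the big worm character and to a bridge.
; When a big worm enters Sphere, a timeline lifts that sphere, angles Stick using the stored starting rotation, then enables physics on Sphere1.
; When a BP_Bridge enters Sphere2, both sticks and the bridge start simulating physics, and the bridge becomes very heavy after a short delay.
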(event OnComponentBeginOverlap(Sphere)
  (params (OverlappedComponent :type Primitive%20Component%20Object%20Reference) (OtherActor :type Actor%20Object%20Reference) (OtherComp :type Primitive%20Component%20Object%20Reference) (OtherBodyIndex :type Integer) (bFromSweep :type Boolean) (SweepResult :type Hit%20Result%20Structure%20%28by%20ref%29))
  (bind _sphere (Variables|Default|GetSphere))
  (bind __startingrotation (Variables|Default|Get_startingRotation))
  (bind _returnvalue (Transformation|GetWorldLocation _sphere))
  ;[1 1 1] Moving up the leaf and rotate the sticka
  (bind _asthird_person_character (Utilities|Casting|CastToThirdPersonCharacter OtherActor))
  (if (Variables|/Game/ThirdPersonBP/Blueprints/ThirdPersonCharacter.ThirdPersonCharacter_C|GetIsBigWorm _asthird_person_character)
    (bind _move (Timeline|MoveUp Play)
      (:Update
        (Transformation|SetWorldLocation (Variables|Default|GetSphere) (Math|Vector|Lerp(Vector) (Transformation|GetWorldLocation _sphere) (Math|Vector|MakeVector (.x _returnvalue) (.y _returnvalue) (Variables|Default|Get_leafDistance)) _move) false false)
        (Transformation|SetWorldRotation (Variables|Default|Getstick) (Math|Rotator|MakeRotator (.roll __startingrotation) (Variables|Default|Get_stickAngle) (.yaw __startingrotation)) false false))
      (:Finished
        (Physics|SetSimulatePhysics (Variables|Default|GetSphere1) true)))))

(event OnComponentBeginOverlap(Sphere2)
  (params (OverlappedComponent :type Primitive%20Component%20Object%20Reference) (OtherActor :type Actor%20Object%20Reference) (OtherComp :type Primitive%20Component%20Object%20Reference) (OtherBodyIndex :type Integer) (bFromSweep :type Boolean) (SweepResult :type Hit%20Result%20Structure%20%28by%20ref%29))
  ;[1 1 1] Set the physics for stick and bridge
  (bind _asbp_bridge (Utilities|Casting|CastToBP_Bridge OtherActor))
  (if (Variables|/Game/Blueprint/BP_Bridge.BP_Bridge_C|GetIsBridge _asbp_bridge)
    (Physics|SetSimulatePhysics (Variables|Default|Getstick) true)
    (Physics|SetSimulatePhysics (Variables|Default|Getstick1) true)
    (Physics|SetSimulatePhysics (Variables|/Game/Blueprint/BP_Bridge.BP_Bridge_C|GetBridge _asbp_bridge) true)
    (Utilities|FlowControl|Delay 0.2)
    (Class|PrimitiveComponent|SetMassOverrideinKg (Variables|/Game/Blueprint/BP_Bridge.BP_Bridge_C|GetBridge _asbp_bridge) "None" 1e+04 true)))

(fn ConstructionScript
  (Variables|Default|Set_startingRotation (Transformation|GetActorRotation)))